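; BP_DestroyedTank is the wreck of a destroyed tank that plays destruction effects when it begins play.
; After a brief delay it spawns a BP_RadialForceTank actor at a marker component for a physics impulse.
; It then fires a large explosion, sparks and smoke at scene component locations.
; Sparks and smoke deactivate on separate timers, with smoke lingering longer.
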(event EventBeginPlay
  (bind _post_destruction_vfx (Variables|Default|GetPost%20Destruction%20VFX))
  (bind _returnvalue (Transformation|GetWorldLocation _post_destruction_vfx))
  (Utilities|FlowControl|Delay 0.1)
  (Game|SpawnActorfromClass "/Game/Blueprints/BP_RadialForceTank.BP_RadialForceTank_C" (Math|Conversions|ToTransform(Vector) (Transformation|GetWorldLocation (Variables|Default|GetRadialForceLocation))) "AlwaysSpawn" "MultiplyWithRoot" 0 0)
  (Utilities|FlowControl|Sequence
    (:then_0
      ;[1 1 1] Explosion VFX
      (Effects|SpawnEmitteratLocation "/Game/Realistic_Starter_VFX_Pack_Vol2/Particles/Explosion/P_Explosion_Big_B.P_Explosion_Big_B" (Transformation|GetWorldLocation (Variables|Default|GetMainExplosionLocation)) "0, 0, 0" "2.000000,2.000000,2.000000"))
    (:then_1
      ;[1 1 1] Sparks VFX
      (bind _returnvalue_2 (Niagara|SpawnSystematLocation "/Game/Realistic_Starter_VFX_Pack_Vol2/Particles/Sparks/P_Sparks_D_Converted.P_Sparks_D_Converted" _returnvalue))
      (Utilities|FlowControl|Delay 3e+01)
      (Components|Activation|Deactivate _returnvalue_2))
    (:then_2
      ;[1 1 1] Smoke VFX
      (bind _returnvalue_3 (Effects|SpawnEmitteratLocation "/Game/Realistic_Starter_VFX_Pack_Vol2/Particles/Smoke/P_Smoke_B.P_Smoke_B" _returnvalue))
      (Utilities|FlowControl|Delay 9e+01)
      (Components|Activation|Deactivate _returnvalue_3))))

(fn ConstructionScript)