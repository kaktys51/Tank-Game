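; Game mode for a tank game that shows win/lose screens, relays score updates and manages a pre-game lobby.
; PostLogin and OnLogout track controllers and player states, showing the pre-game widget to joiners.
; The ready check calls StartGame even after breaking on an unready player; StartGame is an empty stub.
; SpawnPlayerPawn, uncalled here, possesses pawnless controllers with tanks at PlayerStarts matched by join-list index.
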(event Custom|Start%20Game)

(event EventGameLose
  ;[0.2517 0.2517 0.2517] Game Rules
  (bind _returnvalue (UserInterface|CreateWidget "/Game/Blueprints/Widgets/WBP_LoseScreen.WBP_LoseScreen_C"))
  (UserInterface|Viewport|AddtoViewport _returnvalue 0))

(event EventGameWin
  ;[0.2517 0.2517 0.2517] Game Rules
  (bind _returnvalue (UserInterface|CreateWidget "/Game/Blueprints/Widgets/WBP_WinScreen.WBP_WinScreen_C"))
  (UserInterface|Viewport|AddtoViewport _returnvalue 0))

(event EventScoreUpdate
  ;[0.2517 0.2517 0.2517] Game Rules
  (bind _returnvalue (Class|GameModeBaseFox|GetCurrentScore))
  (Default|CallScoreUpdateDispathcer _returnvalue))

(event EventPostLogin
  (params (NewPlayer :type Player%20Controller%20Object%20Reference))
  ;[1 0.9347 0.5981] Colecting loged players
  (Utilities|Array|Add (Variables|Default|GetAllControllers) NewPlayer)
  (if (Variables|Default|GetbIsPreGameState)
    (bind _asbp_custom_player_controller (Utilities|Casting|CastToBP_CustomPlayerController NewPlayer))
    (bind _asplayer_state_fox (Utilities|Casting|CastToPlayerStateFox (Variables|/Script/Engine.Controller|GetPlayerState _asbp_custom_player_controller)))
    (Utilities|Array|Add (Variables|Default|GetAs%20Player%20State%20Fox) _asplayer_state_fox)
    (Default|DisplayPreGameWidget _asbp_custom_player_controller)))

(event EventOnLogout
  (params (ExitingController :type Controller%20Object%20Reference))
  ;[1 0.9347 0.5981] Colecting loged players
  (bind _asbp_custom_player_controller (Utilities|Casting|CastToBP_CustomPlayerController ExitingController))
  (Utilities|Array|RemoveItem (Variables|Default|GetAllControllers) _asbp_custom_player_controller)
  (bind _asplayer_state_fox (Utilities|Casting|CastToPlayerStateFox (Variables|/Script/Engine.Controller|GetPlayerState _asbp_custom_player_controller)))
  (Utilities|Array|RemoveItem (Variables|Default|GetAs%20Player%20State%20Fox) _asplayer_state_fox))

(event EventCheckAllPlayersReady
  (bind _array_element (Utilities|Array|ForEachLoopwithBreak (Variables|Default|GetAllControllers) :!label _label)
    (:LoopBody
      (bind _asbp_custom_player_controller (Utilities|Casting|CastToBP_CustomPlayerController _array_element))
      (if (not (Variables|/Script/part_3.CustomPlayerController|GetbIsReady _asbp_custom_player_controller))
        (goto _label Break)))
    (:Completed
      (CallFunction|StartGame))))

(fn ConstructionScript)

(fn SpawnPlayerPawn
  (params (PlayerController :type Player%20Controller%20Object%20Reference))
  (bind _allcontrollers (Variables|Default|GetAllControllers))
  (bind _returnvalue (Utilities|Array|FindItem _allcontrollers PlayerController))
  (Utilities|IsValid (Pawn|GetControlledPawn PlayerController)
    (:Is%20Valid
      (return))
    (:Is%20Not%20Valid
      (bind _outactors (Actor|GetAllActorsOfClass "/Script/Engine.PlayerStart"))
      (if (< _returnvalue 0)
        (return)
        (else
          (bind _returnvalue_2 (Game|SpawnActorfromClass "/Game/Blueprints/BP_PlayerTank.BP_PlayerTank_C" (Transformation|GetActorTransform (Utilities|Array|Get(acopy) _outactors _returnvalue)) "AdjustIfPossibleButAlwaysSpawn" "MultiplyWithRoot" 0 0))
          (Pawn|Possess PlayerController _returnvalue_2))))))

(fn ChoosePlayerStart
  (params (Player :type Controller%20Object%20Reference))
  (return 0))