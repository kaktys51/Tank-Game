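; Player-controlled tank pawn for a networked game, handling Enhanced Input movement, look and firing, plus HUD and pause menu.
; Next-tick timers set up input mapping and UI for the local player, and health updates go out through a dispatcher.
; Tick toggles track dust and speed-pitched MetaSound from real velocity locally, or from authority-set SimTankVelocity on simulated clients.
; It also defines fire effects and turret rotation sound, and draws debug health and capsules.
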(event Input|EnhancedActionEvents|EnhancedInputActionIA_MoveForward
  (params (ActionValue :type Float%20%28double-precision%29) (ElapsedSeconds :type Float%20%28double-precision%29) (TriggeredSeconds :type Float%20%28double-precision%29) (InputAction :type Input%20Action%20Object%20Reference :default "/Game/Blueprints/Input/IA_MoveForward.IA_MoveForward"))
  ;[0.5693 0.7885 1] Movement
  (Class|TankPawn|MoveComp ActionValue))

(event Input|EnhancedActionEvents|EnhancedInputActionIA_TunRight
  (params (ActionValue :type Float%20%28double-precision%29) (ElapsedSeconds :type Float%20%28double-precision%29) (TriggeredSeconds :type Float%20%28double-precision%29) (InputAction :type Input%20Action%20Object%20Reference :default "/Game/Blueprints/Input/IA_TunRight.IA_TunRight"))
  ;[0.5693 0.7885 1] Movement
  (Class|TankPawn|TurnComp ActionValue))

(event Input|EnhancedActionEvents|EnhancedInputActionIA_Fire
  (params (ActionValue :type Boolean) (ElapsedSeconds :type Float%20%28double-precision%29) (TriggeredSeconds :type Float%20%28double-precision%29) (InputAction :type Input%20Action%20Object%20Reference :default "/Game/Blueprints/Input/IA_Fire.IA_Fire"))
  ;[1 0.5583 0.5333] Shooting
  (Class|TankPawn|Fire))

(event Input|EnhancedActionEvents|EnhancedInputActionIA_Look
  (params (ActionValue :type Vector%202D%20Structure) (ElapsedSeconds :type Float%20%28double-precision%29) (TriggeredSeconds :type Float%20%28double-precision%29) (InputAction :type Input%20Action%20Object%20Reference :default "/Game/Blueprints/Input/IA_Look.IA_Look"))
  ;[0.5693 0.7885 1] Movement
  (Class|TankPawn|Look (Utilities|Struct|MakeInputActionValue (.x ActionValue) (.y ActionValue) 0.0 "Axis2D")))

(event Input|EnhancedActionEvents|EnhancedInputActionIA_PauseGame
  (params (ActionValue :type Boolean) (ElapsedSeconds :type Float%20%28double-precision%29) (TriggeredSeconds :type Float%20%28double-precision%29) (InputAction :type Input%20Action%20Object%20Reference :default "/Game/Blueprints/Input/IA_PauseGame.IA_PauseGame"))
  (bind _returnvalue (Game|GetPlayerController 0))
  (bind _returnvalue_2 (Game|GetPlayerController 0))
  ;[0.1127 0.09085 0.342] Pause Menu
  (if (not (Variables|Default|GetisPauseMenuOpend?))
    (Variables|Default|SetisPauseMenuOpend? true)
    (bind _returnvalue_3 (UserInterface|CreateWidget "/Game/Blueprints/Widgets/WBP_PauseMenu.WBP_PauseMenu_C" _returnvalue_2))
    (bind _output_get (Variables|Default|SetPauseMenuWiget _returnvalue_3))
    (UserInterface|Viewport|AddtoViewport _output_get 0)
    (Input|SetInputModeGameandUI _returnvalue_2 _output_get "DoNotLock" true false)
    (Game|SetGamePaused true)
    (bind _asbp_custom_player_controller (Utilities|Casting|CastToBP_CustomPlayerController _returnvalue_2))
    (Default|DisableCenteredCursour _asbp_custom_player_controller)
    (Variables|/Script/Engine.PlayerController|SetbShowMouseCursor _asbp_custom_player_controller true)
    (else
      (Variables|Default|SetisPauseMenuOpend? false)
      (Game|SetGamePaused false)
      (Input|SetInputModeGameOnly _returnvalue false)
      (bind _asbp_custom_player_controller_2 (Utilities|Casting|CastToBP_CustomPlayerController _returnvalue))
      (Default|EnableCenteredCursour _asbp_custom_player_controller_2)
      (Variables|/Script/Engine.PlayerController|SetbShowMouseCursor _asbp_custom_player_controller_2 false)
      (Widget|RemovefromParent (Variables|Default|GetPauseMenuWiget)))))

(event EventBeginPlay
  (bind _returnvalue (Game|GetPlayerController 0))
  (Class|KismetSystemLibrary|SetTimerforNextTick 0 "InputSetup")
  (Class|KismetSystemLibrary|SetTimerforNextTick 0 "SetupUI")
  ;[0.4546 0.8965 1] Setting up camera in right direction on client side
  (if (Pawn|IsLocallyControlled)
    (Utilities|IsValid _returnvalue
      (:Is%20Valid
        (Pawn|SetControlRotation _returnvalue (Transformation|GetWorldRotation (Variables|Default|GetCameraStatrtingPoint)))))))

(event Game|Damage|EventAnyDamage
  (params (Damage :type Float%20%28single-precision%29) (DamageType :type Damage%20Type%20Object%20Reference) (InstigatedBy :type Controller%20Object%20Reference) (DamageCauser :type Actor%20Object%20Reference))
  (Development|PrintString "damage"))

(event EventTick
  (params (DeltaSeconds :type Float%20%28single-precision%29))
  (bind _capsulecomponent (Variables|Default|GetCapsuleComponent))
  (bind _returnvalue (Transformation|GetWorldLocation _capsulecomponent))
  (Networking|SwitchHasAuthority
    (:Authority
      (Rendering|Debug|DrawDebugCapsule _returnvalue 1.2e+02 1.2e+02 "0, 0, 0" "(R=1.000000,G=0.000000,B=0.006108,A=1.000000)" 0.0 0.0))
    (:Remote
      (Rendering|Debug|DrawDebugCapsule _returnvalue 1.2e+02 1.2e+02 "0, 0, 0" "(R=0.105738,G=0.090768,B=1.000000,A=1.000000)" 0.0 0.0)))
  (Rendering|Debug|DrawDebugString (Transformation|GetActorLocation) (Utilities|String|Append "Health:" (Utilities|String|ToString(Float) (Variables|/Script/part_3.HealthComponent|GetCurrentHealth (Variables|Default|GetHealthComponent)))) 0 "(R=0.059716,G=0.023065,B=1.000000,A=1.000000)")
  (Networking|SwitchHasAuthority
    (:Authority
      (Variables|Default|SetSimTankVelocity (CallFunction|GetVelocityLenght))
      (if (Pawn|IsLocallyControlled)
        ;[1 0.9667 0.3094] Local Movment VFX/SFX
        (VFX\SFX|TracksVFX)
        (VFX\SFX|TracksSFX)))
    (:Remote
      (if (Pawn|IsLocallyControlled)
        ;[1 0.9667 0.3094] Local Movment VFX/SFX
        (VFX\SFX|TracksVFX)
        (VFX\SFX|TracksSFX)
        (else
          ;[0.526 0.5084 0.1598] Simulated Movment VFX/SFX
          (VFX\SFX|SimTracksVFX)
          (VFX\SFX|SimTracksSFX))))))

(event EventHealthUpdated
  (bind _healthcomponent (Variables|Default|GetHealthComponent))
  ;[0.01468 0.3177 0.005773] Health Update
  (Default|CallHealthDispatcher (Class|HealthComponent|GetCurrentHealth _healthcomponent) (Class|HealthComponent|GetMaxHealth _healthcomponent)))

(event EventFireVSFX
  (bind _fire_vfx (Variables|Default|GetFire%20VFX))
  (bind _returnvalue (Transformation|GetWorldTransform _fire_vfx))
  ;[1 0.5583 0.5333] Shooting VSFX
  (Effects|SpawnEmitteratLocation "/Game/Realistic_Starter_VFX_Pack_Vol2/Particles/Hit/P_CeramicFire.P_CeramicFire" (.location _returnvalue) (.rotation _returnvalue) "3.000000,3.000000,3.000000")
  (Audio|PlaySoundatLocation "/Game/Sound/MS_TankGun.MS_TankGun" (.location (Transformation|GetWorldTransform (Variables|Default|GetTurretMesh))) "0, 0, 0" 1.0 1.0 0.0 0 0 0 0)
  (Class|LegacyCameraShake|StartLegacyCameraShake (Game|GetPlayerCameraManager 0) "/Game/Blueprints/BP_CameraShakeFire.BP_CameraShakeFire_C" 1.0 "CameraLocal" "0, 0, 0"))

(event Input|KeyboardEvents|F
  (params (Key :type Key%20Structure :default "None"))
  (:Pressed
    (if (Variables|/Script/part_3.TankMovementComponent|GetbIsUpdateVisualActive (Variables|Default|GetMovementComponent))
      (Variables|/Script/part_3.TankMovementComponent|SetbIsUpdateVisualActive (Variables|Default|GetMovementComponent) false)
      (else
        (Variables|/Script/part_3.TankMovementComponent|SetbIsUpdateVisualActive (Variables|Default|GetMovementComponent) true)))))

(fn ConstructionScript)

(fn TracksVFX
  (if (> (CallFunction|GetVelocityLenght) (Variables|Default|GetMinVelocityCheck))
    (if (Variables|Default|GetisMovingVFXon?)
      (return)
      (else
        (bind _returnvalue (Effects|SpawnEmitterAttached "/Game/Realistic_Starter_VFX_Pack_Vol2/Particles/Smoke/P_Smoke_C.P_Smoke_C" (Variables|Default|GetMoving%20Dust%20Location) "None"))
        (Variables|Default|SetMoving%20Dust%20Emitter _returnvalue)
        (Variables|Default|SetisMovingVFXon? true)
        (return)))
    (elif (Variables|Default|GetisMovingVFXon?)
      (Variables|Default|SetisMovingVFXon? false)
      (Components|Activation|Deactivate (Variables|Default|GetMoving%20Dust%20Emitter))
      (return)
      (else
        (return)))))

(fn TracksSFX
  (bind _velocity (CallFunction|GetVelocityLenght))
  (LocalVariables|SetTracksVelocity (VFX\SFX|TracksVelocitytoPitch _velocity))
  (if (> _velocity (Variables|Default|GetMinVelocityCheck))
    (if (Variables|Default|GetisMovingSFXon?)
      (Audio|Parameter|SetFloatParameter (Variables|Default|GetTrackSound) "TracksSpeed" (LocalVariables|GetTracksVelocity) :!class /Script/AudioExtensions.AudioParameterControllerInterface)
      (return)
      (else
        (bind _returnvalue (Audio|SpawnSoundAttached "/Game/Sound/MS_TankTracks.MS_TankTracks" (Variables|Default|GetMoving%20Dust%20Location) "None" "0, 0, 0" "0, 0, 0" "KeepRelativeOffset" false 1.0 1.0 0.0 0 0))
        (Variables|Default|SetTrackSound _returnvalue)
        (Variables|Default|SetisMovingSFXon? true)
        (return)))
    (elif (Variables|Default|GetisMovingSFXon?)
      (Variables|Default|SetisMovingSFXon? false)
      (Audio|Components|Audio|FadeOut (Variables|Default|GetTrackSound) 1.5 0.0 "Linear" :!class /Script/Engine.AudioComponent)
      (return)
      (else
        (return)))))

(fn TurretSFX
  (bind _output_get (Variables|Default|SetTurretCurRotator (Transformation|GetWorldRotation (Variables|Default|GetTurretMesh))))
  (if (Utilities|Operators|NotEqual(!=) _output_get (Variables|Default|GetTurretPrevRotator) 0.1)
    (Variables|Default|SetTurretPrevRotator (Variables|Default|GetTurretCurRotator))
    (Variables|Default|GetRotationSound
      (:then
        (return))
      (:else
        (bind _returnvalue (Audio|SpawnSoundAttached "/Game/Sound/MS_TurretRotation.MS_TurretRotation" (Variables|Default|GetTurretMesh) "None" "0, 0, 0" "0, 0, 0" "KeepRelativeOffset" false 1.0 1.0 0.0 0 0))
        (Variables|Default|SetRotationSound _returnvalue)
        (Development|PrintString "Turret rot SFX")
        (return)))
    (else
      (bind _rotationsound (Variables|Default|GetRotationSound)
        (:then
          (Audio|Components|Audio|FadeOut _rotationsound 0.5 0.0 "Linear" :!class /Script/Engine.AudioComponent)
          (return))
        (:else
          (return))))))

(fn GetVelocityLenght
  (bind _output_get (LocalVariables|SetVelocityLenght (Math|Vector|VectorLength (Transformation|GetVelocity))))
  (return _output_get))

(fn TracksVelocitytoPitch
  (params (Velocity :type Float%20%28double-precision%29))
  (bind _result (Math|Float|NegateFloat Velocity)
    (:%20%20
      (return (* (Math|Float|NormalizetoRange _result (LocalVariables|GetTankMaxVelocityNegated) 0.0) (LocalVariables|GetMinPichValue))))))

(fn InputSetup
  (if (Pawn|IsLocallyControlled)
    (bind _asplayer_controller (Utilities|Casting|CastToPlayerController (Pawn|GetController)))
    (Input|AddMappingContext (PlayerController|LocalPlayerSubsystems|GetEnhancedInputLocalPlayerSubsystem _asplayer_controller) "/Game/Blueprints/Input/IMC_TankMovementContext.IMC_TankMovementContext" 0 "(bIgnoreAllPressedKeysUntilRelease=True,bForceImmediately=False,bNotifyUserSettings=False)")
    (bind _asbp_custom_player_controller (Utilities|Casting|CastToBP_CustomPlayerController _asplayer_controller))
    (return)))

(fn SimTracksSFX
  (bind _simtankvelocity (Variables|Default|GetSimTankVelocity))
  (LocalVariables|SetLocal%20Sim%20Tracks%20Velocity (VFX\SFX|TracksVelocitytoPitch _simtankvelocity))
  (if (> _simtankvelocity (Variables|Default|GetMinVelocityCheck))
    (if (Variables|Default|GetisMovingSFXon?)
      (Audio|Parameter|SetFloatParameter (Variables|Default|GetTrackSound) "TracksSpeed" (LocalVariables|GetLocal%20Sim%20Tracks%20Velocity) :!class /Script/AudioExtensions.AudioParameterControllerInterface)
      (return)
      (else
        (bind _returnvalue (Audio|SpawnSoundAttached "/Game/Sound/MS_TankTracks.MS_TankTracks" (Variables|Default|GetMoving%20Dust%20Location) "None" "0, 0, 0" "0, 0, 0" "KeepRelativeOffset" false 1.0 1.0 0.0 0 0))
        (Variables|Default|SetTrackSound _returnvalue)
        (Variables|Default|SetisMovingSFXon? true)
        (return)))
    (elif (Variables|Default|GetisMovingSFXon?)
      (Variables|Default|SetisMovingSFXon? false)
      (Audio|Components|Audio|FadeOut (Variables|Default|GetTrackSound) 1.5 0.0 "Linear" :!class /Script/Engine.AudioComponent)
      (return)
      (else
        (return)))))

(fn SimTracksVFX
  (if (> (Variables|Default|GetSimTankVelocity) (Variables|Default|GetMinVelocityCheck))
    (if (Variables|Default|GetisMovingVFXon?)
      (return)
      (else
        (bind _returnvalue (Effects|SpawnEmitterAttached "/Game/Realistic_Starter_VFX_Pack_Vol2/Particles/Smoke/P_Smoke_C.P_Smoke_C" (Variables|Default|GetMoving%20Dust%20Location) "None"))
        (Variables|Default|SetMoving%20Dust%20Emitter _returnvalue)
        (Variables|Default|SetisMovingVFXon? true)
        (return)))
    (elif (Variables|Default|GetisMovingVFXon?)
      (Variables|Default|SetisMovingVFXon? false)
      (Components|Activation|Deactivate (Variables|Default|GetMoving%20Dust%20Emitter))
      (return)
      (else
        (return)))))

(fn SetupUI
  (if (Pawn|IsLocallyControlled)
    (bind _returnvalue (UserInterface|CreateWidget "/Game/Blueprints/Widgets/UI_TankPlayer.UI_TankPlayer_C" (Game|GetPlayerController 0)))
    (bind _output_get (Variables|Default|SetTankUI _returnvalue))
    (UserInterface|Viewport|AddtoViewport _output_get 0)
    (return)
    (else
      (return))))