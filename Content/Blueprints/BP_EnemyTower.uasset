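; Enemy turret tower pawn that spots pawns and shoots at them, with fire and hit effects.
; On the server, PawnSensing writes sightings to the AI Blackboard as the current or pending target.
; Server Tick calls RotateTurret and Fire while a Blackboard target exists; LoseSight clears that target.
; The construction script matches sight and detection-sphere radii, and Tick draws debug health, muzzle and range.
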(event OnSeePawn(PawnSensing)
  (params (Pawn :type Pawn%20Object%20Reference))
  ;[0.7605 0.5711 1] On pawn sensing, saves target ref locally and at blackboard
  (Networking|SwitchHasAuthority
    (:Authority
      (Utilities|IsValid (Variables|Default|GetTargetPlayerRef)
        (:Is%20Valid
          (AI|Components|Blackboard|SetValueasObject (Variables|/Script/AIModule.AIController|GetBlackboard (Variables|Default|GetAIController)) (Utilities|Name|MakeLiteralName "PendingTargetPlayer") Pawn)
          (Class|TowerPawn|RestartLossSightTimer))
        (:Is%20Not%20Valid
          (AI|Components|Blackboard|SetValueasObject (Variables|/Script/AIModule.AIController|GetBlackboard (Variables|Default|GetAIController)) (Utilities|Name|MakeLiteralName "TargetPlayer") Pawn)
          (CallFunction|UpdateTargetPlayer Pawn))))))

(event EventTick
  (params (DeltaSeconds :type Float%20%28single-precision%29))
  (Rendering|Debug|DrawDebugString (Transformation|GetActorLocation) (Utilities|String|ToString(Float) (Variables|/Script/part_3.HealthComponent|GetCurrentHealth (Variables|Default|GetHealthComponent))) 0 "(R=0.059716,G=0.023065,B=1.000000,A=1.000000)")
  (Rendering|Debug|DrawDebugSphere (Transformation|GetWorldLocation (Variables|Default|GetProjectileSpawnPointFox)) 1e+02 12 "(R=0.157802,G=0.155444,B=1.000000,A=1.000000)" 0.0)
  (Rendering|Debug|DrawDebugSphere (Transformation|GetActorLocation) (Variables|/Script/AIModule.PawnSensingComponent|GetSightRadius (Variables|Default|GetPawnSensing)) 12 "(R=1.000000,G=0.040731,B=0.024152,A=1.000000)" 0.0)
  ;[0.2969 0.03397 0.03298 1 20] Checks for valid target from blackboard and shoots in it
  (Networking|SwitchHasAuthority
    (:Authority
      (Utilities|IsValid (AI|Components|Blackboard|GetValueasObject (Variables|/Script/AIModule.AIController|GetBlackboard (Variables|Default|GetAIController)) (Utilities|Name|MakeLiteralName "TargetPlayer"))
        (:Is%20Valid
          (Class|TurretPawn|RotateTurret (Transformation|GetActorLocation (Variables|Default|GetTargetPlayerRef)))
          (Class|TowerPawn|Fire))
        (:Is%20Not%20Valid
          (Variables|Default|SetTargetPlayerRef 0))))))

(event Collision|EventHit
  (params (MyComp :type Primitive%20Component%20Object%20Reference) (Other :type Actor%20Object%20Reference) (OtherComp :type Primitive%20Component%20Object%20Reference) (bSelfMoved :type Boolean) (HitLocation :type Vector :default "0, 0, 0") (HitNormal :type Vector :default "0, 0, 0") (NormalImpulse :type Vector :default "0, 0, 0") (Hit :type Hit%20Result%20Structure%20%28by%20ref%29))
  (Effects|SpawnEmitteratLocation "/Game/Realistic_Starter_VFX_Pack_Vol2/Particles/Destruction/P_Destruction_Building_A.P_Destruction_Building_A" HitLocation (Math|Rotator|MakeRotfromZ (Math|Vector|NegateVector HitNormal))))

(event EventLoseSight
  ;[0.7605 0.5711 1] Losing Sight over Time
  (AI|Components|Blackboard|ClearValue (Variables|/Script/AIModule.AIController|GetBlackboard (Variables|Default|GetAIController)) (Utilities|Name|MakeLiteralName "TargetPlayer")))

(event EventFireVSFX
  (bind _fire_vfx (Variables|Default|GetFire%20VFX))
  (bind _returnvalue (Transformation|GetWorldTransform _fire_vfx))
  ;[1 0.5583 0.5333] Shooting VSFX
  (Effects|SpawnEmitteratLocation "/Game/Realistic_Starter_VFX_Pack_Vol2/Particles/Hit/P_CeramicFire.P_CeramicFire" (.location _returnvalue) (.rotation _returnvalue) "3.000000,3.000000,3.000000")
  (Audio|PlaySoundatLocation "/Game/Sound/MS_TowerGun.MS_TowerGun" (.location _returnvalue) "0, 0, 0" 1.0 1.0 0.0 0 0 0 0))

(event EventBeginPlay
  ;[0.3989 0.6745 1] Create AIContoller ref
  (Networking|SwitchHasAuthority
    (:Authority
      (bind _asaicontroller (Utilities|Casting|CastToAIController (Pawn|GetController)))
      (Variables|Default|SetAIController _asaicontroller))))

(fn ConstructionScript
  (bind _pawnsensingradius (Variables|Default|GetPawnSensingRadius))
  (Variables|/Script/AIModule.PawnSensingComponent|SetSightRadius (Variables|Default|GetPawnSensing) _pawnsensingradius)
  (Components|Sphere|SetSphereRadius (Variables|Default|GetDetectionSphere) _pawnsensingradius true))

(fn UpdateTargetPlayer
  (params (BlackboardTarget :type Object%20Object%20Reference))
  (bind _aspawn (Utilities|Casting|CastToPawn BlackboardTarget))
  (Variables|Default|SetTargetPlayerRef _aspawn)
  (return))