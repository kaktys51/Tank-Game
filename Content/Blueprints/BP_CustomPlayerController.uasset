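; Player controller for a networked tank game, handling main menu, pre-game UI and pawn spawning.
; BeginPlay shows the main menu on MainMenuMap; otherwise the local controller requests a server spawn through BP_GameModeFox, enables control, turns on turret-to-cursor aiming and hides the cursor.
; The pre-game teams widget appears via an authority-gated display event or player-state receipt once pre-game is flagged.
; Cursor-centering, start-tip and tank HUD logic are disconnected.
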(event Custom|StartGameClosed
  (bind _output_get (Variables|Default|SetIsControllerEnabled true))
  (Class|CustomPlayerController|SetPlayerEnabledState _output_get)
  (bind _astank_pawn (Utilities|Casting|CastToTankPawn (Game|Player|GetPlayerPawn 0)))
  (Class|TankPawn|SetTurretRotationtoCursorState _astank_pawn true)
  (Variables|Default|SetIsCursourCentered true)
  (Variables|/Script/Engine.PlayerController|SetbShowMouseCursor (Game|GetPlayerController 0) false))

(event Custom|DisableCenteredCursour
  (Variables|Default|SetIsCursourCentered false))

(event Custom|EnableCenteredCursour
  (Variables|Default|SetIsCursourCentered true))

(event Custom|Server_SpawnPlayer
  (bind _asbp_game_mode_fox (Utilities|Casting|CastToBP_GameModeFox (Game|GetGameMode)))
  (Default|SpawnPlayerPawn _asbp_game_mode_fox self))

(event Custom|DisplayPreGameWidget
  (Variables|Default|SetisPreGame? true)
  (Networking|SwitchHasAuthority
    (:Authority
      (CallFunction|DisplayPreGameTeamsWidget))))

(event EventTick
  (params (DeltaSeconds :type Float%20%28single-precision%29))
  ;[0.3736 0.4526 1] Locks the cursor position in the center of the screen
)

(event EventPossess
  (params (PossessedPawn :type Pawn%20Object%20Reference)))

(event EventBeginPlay
  (bind _ismainmenu_ (CallFunction|MainMenuCheck))
  (if _ismainmenu_
    (bind _returnvalue (UserInterface|CreateWidget "/Game/Blueprints/Widgets/WBP_MainMenu.WBP_MainMenu_C"))
    (bind _output_get (Variables|Default|SetMainMenu%20Ref _returnvalue))
    (UserInterface|Viewport|AddtoViewport _output_get 0)
    (elif (Pawn|IsLocalPlayerController)
      (CallFunction|ServerSpawnPlayer)
      (bind _output_get_2 (Variables|Default|SetIsControllerEnabled true))
      (Class|CustomPlayerController|SetPlayerEnabledState _output_get_2)
      (bind _astank_pawn (Utilities|Casting|CastToTankPawn (Game|Player|GetPlayerPawn 0)))
      (Class|TankPawn|SetTurretRotationtoCursorState _astank_pawn true)
      (Variables|Default|SetIsCursourCentered true)
      (Variables|/Script/Engine.PlayerController|SetbShowMouseCursor (Game|GetPlayerController 0) false))))

(event EventRecivedPlayerState
  (params (NewPlayerState :type Player%20State%20Fox%20Object%20Reference))
  (Variables|Default|SetPlayer%20State%20Fox%20Ref NewPlayerState)
  (CallFunction|DisplayPreGameTeamsWidget))

(event EventOptionsClosed
  (bind _returnvalue (Game|GetCurrentLevelName true))
  (if (Utilities|Enum|Equal(Enum) _returnvalue "MainMenuMap")
    (UserInterface|Viewport|AddtoViewport (Variables|Default|GetMainMenu%20Ref) 0)))

(fn ConstructionScript)

(fn CenterCursour
  (bind (_sizex _sizey) (HUD|GetViewportSize))
  (if (Variables|Default|GetIsCursourCentered)
    (Class|PlayerController|SetMouseLocation (/ _sizex 2) (+ (/ _sizey 2) -100))
    (return)
    (else
      (return))))

(fn MainMenuCheck
  (bind _returnvalue (Game|GetCurrentLevelName true))
  (return (Utilities|Enum|Equal(Enum) _returnvalue "MainMenuMap")))

(fn DisplayPreGameTeamsWidget
  (if (Variables|Default|GetisPreGame?)
    (bind _returnvalue (UserInterface|CreateWidget "/Game/Blueprints/Widgets/WBP_PreGameTeams.WBP_PreGameTeams_C"))
    (bind _output_get (Variables|Default|SetPre%20Game%20Ref _returnvalue))
    (UserInterface|Viewport|AddtoViewport _output_get 0)))